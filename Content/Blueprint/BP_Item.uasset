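; BP_Item is an item Blueprint with an elemental type, a damage value and a name.
; On BeginPlay it prints its element and the GetDamage result against a fixed "air" victim as a debug message.
; GetDamage ignores the victim's element and applies no modifier, only returning base Damage in its element-index check.
; A separate Constructor function picks a random name from a hardcoded list, with an index range one past the end.
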(event `self.ReceiveBeginPlay`
  (bind _damage (`self.GetDamage` "NewEnumerator0"))
  (`KismetSystemLibrary.PrintString` (`KismetStringLibrary.Concat_StrStr` "Our element type is" (`|GetEnumeratorNameAsString` (`self.ElementalType`)) ", victim is air, damage =" (`KismetStringLibrary.Conv_IntToString` _damage))))

(fn `Constructor`
  (bind _array (`|MakeArray` "Ash" "Sam" "Grace" "Park"))
  (`KismetArrayLibrary.Array_Shuffle` _array)
  (set `self.Name` (`|GetArrayItem` _array (`KismetMathLibrary.RandomIntegerInRange` 0 (`KismetArrayLibrary.Array_Length` _array)))))

(fn `GetDamage`
  (params (VictimElementalType :type "/Game/Blueprint/ElementalType Enum" :default "NewEnumerator0"))
  (returns (Damage :type Integer))
  (set `self.Return Damage` (`self.Damage`))
  (if (== (`KismetMathLibrary.Conv_ByteToInt` (`self.ElementalType`)) 5)
    (set `self.Return Damage` (`self.Damage`))
    (return (`self.Return Damage`))))

(fn `UserConstructionScript`)