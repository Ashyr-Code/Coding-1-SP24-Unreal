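; Enemy actor that dies when the third-person player character touches its capsule.
; On BeginPlay it applies the team material to its cylinder, or a random one from a shuffled array, and picks a random name if none is set, printing debug strings.
; A looping 0.2-second Delay polls Health and destroys the actor at zero or below; capsule overlap with the player sets Health negative.
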(event `self.ReceiveBeginPlay`
  (bind _names (`self.Names`))
  (bind _color_array (`self.Color Array`))
  (`|ExecutionSequence`
    (:`then_0`
      (`KismetSystemLibrary.Delay` 0.2 :!label _label)
      (if (<= (`self.Health`) 0.0)
        (`self.K2_DestroyActor`)
        (else
          (goto _label))))
    (:`then_1`
      (`/Engine/EditorBlueprintResources/StandardMacros.IsValid` (`self.Enemy Team Material`)
        (:`Is Valid`
          (`KismetSystemLibrary.PrintString` "Hello")
          (`PrimitiveComponent.SetMaterial` (`self.Cylinder`) 0 (`self.Enemy Team Material`)))
        (:`Is Not Valid`
          (`KismetSystemLibrary.PrintString` "Hello")
          (`KismetArrayLibrary.Array_Shuffle` _color_array)
          (`PrimitiveComponent.SetMaterial` (`self.Cylinder`) 0 (`|GetArrayItem` _color_array)))))
    (:`then_2`
      (if (== (`self.Enemy Name`) "None")
        (`KismetArrayLibrary.Array_Shuffle` _names)
        (set `self.Enemy Name` (`|GetArrayItem` _names)))
      (`KismetSystemLibrary.PrintString` (`KismetStringLibrary.Concat_StrStr` (`KismetStringLibrary.Conv_NameToString` (`self.Enemy Name`)))))))

(event `self.Capsule.OnComponentBeginOverlap`
  (params (OverlappedComponent :type "PrimitiveComponent Object Reference") (OtherActor :type "Actor Object Reference") (OtherComp :type "PrimitiveComponent Object Reference") (OtherBodyIndex :type Integer) (bFromSweep :type Boolean) (SweepResult :type "HitResult Structure (by ref)"))
  (cast `/Game/ThirdPerson/Blueprints/BP_ThirdPersonCharacter` OtherActor)
  (set `self.Health` -1.0))

(fn `UserConstructionScript`)