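; Enemy spawn manager Blueprint that gathers all Spawner actors on BeginPlay, prints their count and populates them with enemies.
; SpawnEnemies rolls per spawner, giving each roughly a one-in-five chance to spawn an Enemy at its transform.
; CheckEnemyCount re-calls itself through a short Delay, but its actor query has no class and its branch condition is fixed true, so it never respawns enemies.
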(event `self.ReceiveBeginPlay`
  (bind _outactors (`GameplayStatics.GetAllActorsOfClass` "/Game/Blueprint/Spawner.Spawner_C"))
  (`KismetSystemLibrary.PrintString` (`KismetStringLibrary.Concat_StrStr` "There are " (`KismetStringLibrary.Conv_IntToString` (`KismetArrayLibrary.Array_Length` _outactors))))
  (`self.Spawn Enemies`)
  (`self.Check Enemy Count`))

(event `Spawn Enemies`
  (for _array_element (stale `self.ReceiveBeginPlay` _outactors)
    (if (< 0.8 (`KismetMathLibrary.RandomFloat`))
      (`|SpawnActorFromClass` "/Game/Blueprint/Enemy.Enemy_C" (`self.GetTransform` _array_element) "Undefined" "MultiplyWithRoot" null null))))

(event `Check Enemy Count`
  (bind _outactors (`GameplayStatics.GetAllActorsOfClass` null))
  (if (not true)
    (`self.Spawn Enemies`))
  (`KismetSystemLibrary.Delay` 0.2)
  (`self.Check Enemy Count`))

(fn `UserConstructionScript`)